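; BP_Key is a pickable key that registers its class in the ThirdPersonCharacter's parallel Inventory and InventoryCount arrays.
; Beginning an overlap runs Interaction and prints a debug value, while ending the overlap destroys the key.
; A new class seeds its count with its array index, while a repeat sets its slot to the first slot's count plus one.
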(event Custom|Interaction
  (bind _self self)
  (bind _returnvalue (Utilities|GetClass _self))
  (bind _asthird_person_character (Utilities|Casting|CastToThirdPersonCharacter (Game|GetPlayerCharacter 0)))
  (if (Utilities|Array|ContainsItem (Variables|/Game/ThirdPersonBP/Blueprints/ThirdPersonCharacter.ThirdPersonCharacter_C|GetInventory _asthird_person_character) _returnvalue)
    (Utilities|Array|SetArrayElem (Variables|/Game/ThirdPersonBP/Blueprints/ThirdPersonCharacter.ThirdPersonCharacter_C|GetInventoryCount _asthird_person_character) (Utilities|Array|FindItem (Variables|/Game/ThirdPersonBP/Blueprints/ThirdPersonCharacter.ThirdPersonCharacter_C|GetInventory _asthird_person_character) _returnvalue) (+ (Utilities|Array|Get(acopy) (Variables|/Game/ThirdPersonBP/Blueprints/ThirdPersonCharacter.ThirdPersonCharacter_C|GetInventoryCount _asthird_person_character)) 1))
    (else
      (bind _returnvalue_2 (Utilities|Array|Add (Variables|/Game/ThirdPersonBP/Blueprints/ThirdPersonCharacter.ThirdPersonCharacter_C|GetInventory _asthird_person_character) _returnvalue))
      (bind _returnvalue_3 (Utilities|Array|Add (Variables|/Game/ThirdPersonBP/Blueprints/ThirdPersonCharacter.ThirdPersonCharacter_C|GetInventoryCount _asthird_person_character) _returnvalue_2)))))

(event Collision|EventActorBeginOverlap
  (params (OtherActor :type Actor%20Object%20Reference))
  (CallFunction|Interaction)
  (Development|PrintString (Utilities|String|ToString(Integer) (stale Custom|Interaction _returnvalue_3)) true true "(R=0.000000,G=0.660000,B=1.000000,A=1.000000)" 1e+02))

(event Collision|EventActorEndOverlap
  (params (OtherActor :type Actor%20Object%20Reference))
  (Actor|DestroyActor))

(fn ConstructionScript)