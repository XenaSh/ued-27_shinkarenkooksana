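; BP_Door_Child is a child door Blueprint that reacts when a ThirdPersonCharacter overlaps it with fewer than three inventory items.
; It disables its own input, computes the missing count and shows one of three TextRender messages for that count for two seconds.
; Tick prints the remaining count on screen as debug output.
; This graph takes no action when the character has three or more items.
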(event EventBeginPlay)

(event Collision|EventActorBeginOverlap
  (params (OtherActor :type Actor%20Object%20Reference))
  (bind _asthird_person_character (Utilities|Casting|CastToThirdPersonCharacter OtherActor))
  (if (not (>= (Utilities|Array|Length (Variables|/Game/ThirdPersonBP/Blueprints/ThirdPersonCharacter.ThirdPersonCharacter_C|GetInventoryCount _asthird_person_character)) 3))
    (Input|DisableInput 0)
    (bind _output_get (Variables|Default|SetRemain (- 3 (Utilities|Array|Length (Variables|/Game/ThirdPersonBP/Blueprints/ThirdPersonCharacter.ThirdPersonCharacter_C|GetInventoryCount _asthird_person_character)))))
    (switch int _output_get
      (:1
        (Rendering|SetVisibility (Variables|Default|GetTextRender3) true false)
        (Utilities|FlowControl|Delay 2.0)
        (Rendering|SetVisibility (Variables|Default|GetTextRender3) false false))
      (:2
        (Rendering|SetVisibility (Variables|Default|GetTextRender2) true false)
        (Utilities|FlowControl|Delay 2.0)
        (Rendering|SetVisibility (Variables|Default|GetTextRender2) false false))
      (:3
        (Rendering|SetVisibility (Variables|Default|GetTextRender1) true false)
        (Utilities|FlowControl|Delay 2.0)
        (Rendering|SetVisibility (Variables|Default|GetTextRender1) false false)))))

(event EventTick
  (params (DeltaSeconds :type Float%20%28single-precision%29))
  (Development|PrintString (Utilities|String|ToString(Integer) (stale Collision|EventActorBeginOverlap _output_get)) true true "(R=0.049932,G=1.000000,B=0.000000,A=1.000000)" DeltaSeconds))

(fn ConstructionScript
  (|CallParentFunction))