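; Interactive door Blueprint that swings open away from the player and closes again on the OpenDoor input.
; A box overlap enables input and shows a text prompt only while in range.
; A dot product of player-to-door direction and door forward selects the yaw sign, and a timeline lerps the mesh rotation, reversing to close.
; Disconnected leftover rotation attempts remain in the graph.
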(event OnComponentBeginOverlap(Box)
  (params (OverlappedComponent :type Primitive%20Component%20Object%20Reference) (OtherActor :type Actor%20Object%20Reference) (OtherComp :type Primitive%20Component%20Object%20Reference) (OtherBodyIndex :type Integer) (bFromSweep :type Boolean) (SweepResult :type Hit%20Result%20Structure%20%28by%20ref%29))
  ;[1 1 1] Overlap
  (Input|EnableInput (Game|GetPlayerController 0))
  (Rendering|SetVisibility (Variables|Default|GetTextRender) true false))

(event OnComponentEndOverlap(Box)
  (params (OverlappedComponent :type Primitive%20Component%20Object%20Reference) (OtherActor :type Actor%20Object%20Reference) (OtherComp :type Primitive%20Component%20Object%20Reference) (OtherBodyIndex :type Integer))
  ;[1 1 1] Overlap
  (Input|DisableInput (Game|GetPlayerController 0))
  (Rendering|SetVisibility (Variables|Default|GetTextRender) false false))

(event Input|ActionEvents|InputActionOpenDoor
  (params (Key :type Key%20Structure :default "None"))
  (bind _defaultsceneroot1 (Variables|Default|GetDefaultSceneRoot1))
  ;[1 1 1] DoorOpensAway
  (:Pressed
    (if (Variables|Default|GetIsClosed)
      (Variables|Default|SetIsClosed false)
      (Variables|Default|SetDotProduct (Math|Vector|DotProduct (Math|Vector|Normalize (- (Transformation|GetWorldLocation _defaultsceneroot1) (Transformation|GetActorLocation (Game|GetPlayerCharacter 0)))) (Math|Vector|GetForwardVector _defaultsceneroot1)))
      (bind (_direction _newtrack_0) (Timeline|Timeline_0 Play)
        (:Update
          (Transformation|SetRelativeRotation (Variables|Default|GetSM_Door) (Math|Rotator|MakeRotator 0.0 0.0 (Math|Float|Lerp 0.0 (Math|Float|SelectFloat 9e+01 -9e+01 (>= (Variables|Default|GetDotProduct) 0.0)) _newtrack_0)) false false))
        (:Finished
          (switch Utilities|FlowControl|Switch|SwitchonETimelineDirection _direction
            (:Backward
              (Variables|Default|SetIsClosed true)))))
      (else
        (Timeline|Timeline_0 Reverse)))))

(fn ConstructionScript)